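; Test Blueprint for layered dynamic music, driven by the MSDynamicMusic audio component.
; InitializeMusic assigns four wave parameters and starts playback, while UpdateMusicVolume sets a float volume parameter for each layer.
; BeginPlay loads Vampire calm and fleeting tracks into layers 1 and 3, then raises the volume of layers 1 and 4, although layer 4 has no wave assigned.
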(event `self.ReceiveBeginPlay`
  (`self.Initialize Music` "/Game/Taylor/Audio/vampire_calm.vampire_calm" null "/Game/Taylor/Audio/vampire_fleeting.vampire_fleeting")
  (`self.Update Music Volume` 1.0 0.0 0.0 1.0))

(fn `Initialize Music`
  (params (Layer1 :type "SoundWave Object Reference") (Layer2 :type "SoundWave Object Reference") (Layer3 :type "SoundWave Object Reference") (Layer4 :type "SoundWave Object Reference"))
  (`AudioComponent.SetWaveParameter` (`self.MS_DynamicMusic`) "Layer1" Layer1)
  (`AudioComponent.SetWaveParameter` (`self.MS_DynamicMusic`) "Layer2" Layer2)
  (`AudioComponent.SetWaveParameter` (`self.MS_DynamicMusic`) "Layer3" Layer3)
  (`AudioComponent.SetWaveParameter` (`self.MS_DynamicMusic`) "Layer4" Layer4)
  (`AudioComponent.Play` (`self.MS_DynamicMusic`) 0.0))

(fn `Update Music Volume`
  (params (Volume1 :type "Float (double-precision)") (Volume2 :type "Float (double-precision)") (Volume3 :type "Float (double-precision)") (Volume4 :type "Float (double-precision)"))
  (bind _ms_dynamicmusic (`self.MS_DynamicMusic`))
  (`AudioParameterControllerInterface.SetFloatParameter` _ms_dynamicmusic "Volume1" Volume1)
  (`AudioParameterControllerInterface.SetFloatParameter` _ms_dynamicmusic "Volume2" Volume2)
  (`AudioParameterControllerInterface.SetFloatParameter` _ms_dynamicmusic "Volume3" Volume3)
  (`AudioParameterControllerInterface.SetFloatParameter` _ms_dynamicmusic "Volume4" Volume4))

(fn `UserConstructionScript`)