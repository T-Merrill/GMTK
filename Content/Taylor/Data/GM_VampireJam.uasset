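; Game mode for a vampire game that runs one timed night, from player spawn to summary screen.
; BeginPlay spawns and possesses the vampire, near a random TargetPoint after early nights, raises the blood target, restores blood-stain decals and creates the HUD.
; A timer, extended by the NightDuration upgrade, ends the night, updates the high score and shows the summary.
; A fleeing-human counter crossfades music layers through timelines as panic starts and stops.
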(event `self.ReceiveBeginPlay`
  ;[0 0 0] Custom Spawn
  (bind _aspc_vampire_controller (cast `/Game/Taylor/Data/PC_VampireController` (`GameplayStatics.GetPlayerController` 0)))
  (bind _output_get (set `self.As PC Vampire Controller` _aspc_vampire_controller))
  (`Controller.UnPossess` _output_get)
  (bind _spawn_location (`self.Get Spawn Point`))
  (bind _returnvalue (`|SpawnActorFromClass` "/Game/Taylor/Mechanics/BP_VampireCharacter.BP_VampireCharacter_C" (`KismetMathLibrary.MakeTransform` (`KismetMathLibrary.MakeVector` (.x _spawn_location) (.y _spawn_location) 92.0)) "AlwaysSpawn" "MultiplyWithRoot" null null))
  (`Controller.Possess` (`self.As PC Vampire Controller`) _returnvalue)
  (`|ExecutionSequence`
    (:`then_0`
      ;[0 0 0] Variable Setup
      (bind _asgi_game_instance (cast `/Game/Taylor/Data/GI_GameInstance` (`GameplayStatics.GetGameInstance`)))
      (set `self.As GI Game Instance` _asgi_game_instance)
      (set `/Game/Taylor/Data/GI_GameInstance.Target Blood` (+ (`/Game/Taylor/Data/GI_GameInstance.Target Blood` (`self.As GI Game Instance`)) 5) (`self.As GI Game Instance`))
      (`/Game/Taylor/Data/GI_GameInstance.Update Background Music` (`self.As GI Game Instance`))
      (set `self.Fleeing Humans` 0)
      (`/Game/Taylor/Data/GI_GameInstance.Update Volume` (`self.As GI Game Instance`) 1.0 1.0 0.0 0.0)
      ;[0 0 0] Spawn Blood Stains
      (for _array_element (`/Game/Taylor/Data/GI_GameInstance.Blood Stain Transforms` (`self.As GI Game Instance`))
        (`GameplayStatics.SpawnDecalAtLocation` "/Game/Taylor/Materials/M_BloodStain.M_BloodStain" (100.0 100.0 100.0) (.location _array_element) (.rotation _array_element)))
      ;[0 0 0] Check if Player Has Purchased Extra Time
      (if (`KismetArrayLibrary.Array_Contains` (`/Game/Taylor/Data/GI_GameInstance.Purchased Upgrades` (`self.As GI Game Instance`)) "NightDuration")
        (set `self.Night Duration Seconds` 70.0)
        (else
          (set `self.Night Duration Seconds` 60.0)))
      (bind _returnvalue_2 (`KismetSystemLibrary.K2_SetTimerDelegate` (delegate `End Night`) (`self.Night Duration Seconds`)))
      (set `self.Timer Handle` _returnvalue_2))
    (:`then_1`
      ;[0 0 0] Reset NightScore
      (set `/Game/Taylor/Data/GI_GameInstance.Night Score` 0 (`self.As GI Game Instance`))
      ;[0 0 0] Initialize New HUD
      (bind _returnvalue_3 (`|CreateWidget` "/Game/Taylor/UI/HUD/WBP_HUD.WBP_HUD_C"))
      (bind _output_get_2 (set `self.HUD` _returnvalue_3))
      (`UserWidget.AddToViewport` _output_get_2 0))))

(event `End Night`
  ;[0 0 0] Level Complete
  ;;[0 0 0] Evaluate HighScore
  (if (> (`/Game/Taylor/Data/GI_GameInstance.Night Score` (`self.As GI Game Instance`)) (`/Game/Taylor/Data/GI_GameInstance.High Score` (`self.As GI Game Instance`)))
    (set `/Game/Taylor/Data/GI_GameInstance.High Score` (`/Game/Taylor/Data/GI_GameInstance.Night Score` (`self.As GI Game Instance`)) (`self.As GI Game Instance`))
    (bind _asbp_vampire_character (cast `/Game/Taylor/Mechanics/BP_VampireCharacter` (`GameplayStatics.GetPlayerCharacter` 0)))
    (set `/Game/Taylor/Mechanics/BP_VampireCharacter.New High Score?` true _asbp_vampire_character))
  (bind _returnvalue (`|CreateWidget` "/Game/Taylor/UI/NightSummary/WBP_NightSummary.WBP_NightSummary_C"))
  (bind _output_get (set `self.Night Summary` _returnvalue))
  (`UserWidget.AddToViewport` _output_get 0)
  (`/Game/Taylor/Data/PC_VampireController.Set UI Active` (`self.As PC Vampire Controller`) _returnvalue)
  (set `/Game/Taylor/Data/PC_VampireController.Active Blocking Widget?` true (`self.As PC Vampire Controller`)))

(event `Register Fleeing Human`
  (bind _result (`/Engine/EditorBlueprintResources/StandardMacros.IncrementInt` (`self.Fleeing Humans`))
    (:`  `
      (`KismetSystemLibrary.PrintString` (`KismetStringLibrary.Concat_StrStr` "Register: " (`KismetStringLibrary.Conv_IntToString` _result)) true true (struct :`G` 0.66 :`B` 1.0 :`A` 1.0) 10.0)
      (if (== _result 1)
        (bind (_direction _newtrack_0) (`Timeline|MusicFade` :!via `PlayFromStart`)
          (:`Update`
            (`/Game/Taylor/Data/GI_GameInstance.Update Volume` (`self.As GI Game Instance`) 1.0 (- 1.0 _newtrack_0) _newtrack_0 0.0)))))))

(event `Unregister Fleeing Human`
  (bind _output_get (set `self.Fleeing Humans` (`KismetMathLibrary.Clamp` (- (`self.Fleeing Humans`) 1) 0 999)))
  (`KismetSystemLibrary.PrintString` (`KismetStringLibrary.Concat_StrStr` "Unregister: " (`KismetStringLibrary.Conv_IntToString` _output_get)) true true (struct :`G` 0.66 :`B` 1.0 :`A` 1.0) 10.0)
  (if (== _output_get 0)
    (bind (_direction _newtrack_0) (`Timeline|Timeline` :!via `PlayFromStart`)
      (:`Update`
        (`/Game/Taylor/Data/GI_GameInstance.Update Volume` (`self.As GI Game Instance`) 1.0 _newtrack_0 (- 1.0 _newtrack_0) 0.0)))))

(fn `Get Spawn Point`
  (returns (`Spawn Location` :type "Vector Structure"))
  (bind _asgi_game_instance (cast `/Game/Taylor/Data/GI_GameInstance` (`GameplayStatics.GetGameInstance`)))
  ;[0 0 0] First Night Only
  (if (not (<= (`/Game/Taylor/Data/GI_GameInstance.Target Blood` _asgi_game_instance) 5))
    ;[0 0 0] Spawn Somewhere Else
    (`KismetArrayLibrary.Array_Clear` (`self.Spawn Points`))
    (bind _outactors (`GameplayStatics.GetAllActorsOfClass` "/Script/Engine.TargetPoint"))
    (bind _output_get (set `self.Spawn Points` _outactors))
    (bind _randomlocation (`NavigationSystemV1.K2_GetRandomLocationInNavigableRadius` (`self.K2_GetActorLocation` (`KismetArrayLibrary.Array_Random` _output_get)) 0.0 null null))
    (return _randomlocation)))

(fn `UserConstructionScript`)