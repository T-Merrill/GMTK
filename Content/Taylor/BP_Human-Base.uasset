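; Base human NPC for a vampire game that walks toward a random building and serves as a source of blood.
; On BeginPlay it picks a random actor tagged "Building" as its target and uses AI MoveTo toward that building's box component.
; Interact adds its BloodValue to GM_VampireJam and destroys the human.
; The construction script applies the WalkSpeed variable to character movement.
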(event `self.ReceiveBeginPlay`
  ;[0 0 0] Pick a random building index & Set Target Building
  (bind _outactors (`GameplayStatics.GetAllActorsWithTag` "Building"))
  (bind _asbp_building__base (cast `/Game/Taylor/BP_Building-Base` (`|GetArrayItem` _outactors (`KismetMathLibrary.RandomIntegerInRange` 0 (`KismetArrayLibrary.Array_LastIndex` _outactors)))))
  (bind _output_get (set `self.Target Building` _asbp_building__base))
  (`|AIMoveTo` self (`SceneComponent.K2_GetComponentLocation` (`self.GetComponentByClass` _output_get "/Script/Engine.BoxComponent")) null 0.0))

(event `/Game/Taylor/BPI_Interactable.Interact`
  (params (Instigator :type "Actor Object Reference"))
  (bind _asgm_vampire_jam (cast `/Game/Taylor/GM_VampireJam` (`GameplayStatics.GetGameMode`))
    (:`then`
      (`/Game/Taylor/GM_VampireJam.Add Blood` _asgm_vampire_jam (`self.Blood Value`))
      (`self.K2_DestroyActor` self))
    (:`CastFailed`
      ;[1 1 0] DEBUG
      (`KismetSystemLibrary.PrintString` (`KismetStringLibrary.Concat_StrStr` "[BP_Human-Parent] " "Cast " "'Get Game Mode' " "to " " 'GM_VampireJam' " "FAILED")))))

(fn `UserConstructionScript`
  (set `CharacterMovementComponent.MaxWalkSpeed` (`self.Walk Speed`) (`self.CharacterMovement`)))