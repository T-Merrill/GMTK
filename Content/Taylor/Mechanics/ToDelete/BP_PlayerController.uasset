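; Player controller that handles input and menu flow, from pausing to level complete, game complete and losing.
; On BeginPlay it adds the input mapping context and turns the pawn toward the game manager's PlayerLookTarget.
; A held input broadcasts candy shown and hidden, while another toggles the pause menu unless an end screen blocks it.
; End events spawn their widgets, and shared helpers switch input mode, cursor and game pause.
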(event `self.ReceiveBeginPlay`
  (bind _returnvalue (`GameplayStatics.GetPlayerPawn` 0))
  ;[0 0 0] Variable Setup
  (`EnhancedInputSubsystemInterface.AddMappingContext` (subsystem `EnhancedInputLocalPlayerSubsystem`) null 0 (struct))
  (bind _asgm_gameplay (cast `` (`GameplayStatics.GetGameMode`)))
  (set `self.As GameMode` null _asgm_gameplay)
  ;[0 0 0] Set Player Camera Rotation
  (bind _returnvalue_2 (`GameplayStatics.GetActorOfClass` null))
  (set `self.GameManager` null _returnvalue_2)
  (`self.K2_SetActorRotation` _returnvalue (`KismetMathLibrary.FindLookAtRotation` (`self.K2_GetActorLocation` _returnvalue) (`self.K2_GetActorLocation` (`/Game/Taylor/Mechanics/ToDelete/BP_PlayerController.PlayerLookTarget` (`.GameManager` (`self.GameManager`))))) false))

(event `EnhancedInput|`
  (params (ActionValue :type Boolean) (ElapsedSeconds :type "Float (double-precision)") (TriggeredSeconds :type "Float (double-precision)"))
  ;[0 0 0] Player Input Handling
  ;;[0 0 0] Control Candy
  (:`Started`
    (`self.CandyShown`))
  (:`Completed`
    (`self.CandyHidden`)))

(event `EnhancedInput|`
  (params (ActionValue :type Boolean) (ElapsedSeconds :type "Float (double-precision)") (TriggeredSeconds :type "Float (double-precision)"))
  ;[0 0 0] Player Input Handling
  ;;[0 0 0] Pause Game
  (:`Triggered`
    (if (`self.Active Blocking Widget?`)
      _
      (elif (not (`self.PauseMenuOpen?`))
        ;;;[0 0 0] Create Pause Menu
        (bind _returnvalue (`|CreateWidget` null))
        (bind (_output_get _output_get_2) (set `self.Pause Menu` null _returnvalue))
        (`UserWidget.AddToViewport` _output_get_2 0)
        (`self.Set UI Active` _output_get_2)
        (set `self.PauseMenuOpen?` true)
        (else
          ;;;[0 0 0] Exit Pause Menu
          (`self.Set Gameplay Active`)
          (set `self.PauseMenuOpen?` false)
          (`Widget.RemoveFromParent` (`.Pause Menu` (`self.Pause Menu`))))))))

(event `Level Complete`
  ;[0 0 0] On Level Complete
  (`self.Cleanup HUD` (`.As GameMode` (`self.As GameMode`)))
  (bind _returnvalue (`|CreateWidget` "/Game/Taylor/UI/NightSummary/WBP_NightSummary.WBP_NightSummary_C"))
  (set `self.Level Complete Widget Ref` _returnvalue)
  (`UserWidget.AddToViewport` _returnvalue 0)
  (`self.Set UI Active` _returnvalue)
  (set `self.Active Blocking Widget?` true))

(event `On Game Complete`
  ;[0 0 0] On Game Complete
  (bind _returnvalue (`|CreateWidget` "/Game/Taylor/UI/GameComplete/WBP_GameComplete.WBP_GameComplete_C"))
  (`UserWidget.AddToViewport` _returnvalue 0)
  (`self.Set UI Active` null)
  (set `self.Active Blocking Widget?` true))

(event `On Lose Game`
  ;[0 0 0] On Lose Game
  (bind _returnvalue (`|CreateWidget` "/Game/Taylor/UI/LoseMenu/WBP_LoseMenu.WBP_LoseMenu_C"))
  (`UserWidget.AddToViewport` _returnvalue 0)
  (`self.Set UI Active` null)
  (set `self.Active Blocking Widget?` true))

(fn `Set Gameplay Active`
  (`WidgetBlueprintLibrary.SetInputMode_GameOnly` self)
  (set `PlayerController.bShowMouseCursor` false (`GameplayStatics.GetPlayerController` 0))
  (`GameplayStatics.SetGamePaused` false))

(fn `Set UI Active`
  (params (`Menu Ref` :type "Widget Object Reference"))
  (bind _returnvalue (`GameplayStatics.GetPlayerController` 0))
  (`WidgetBlueprintLibrary.SetInputMode_UIOnlyEx` _returnvalue `Menu Ref`)
  (set `PlayerController.bShowMouseCursor` true _returnvalue)
  (`GameplayStatics.SetGamePaused` true))

(fn `UserConstructionScript`)