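; Gameplay game mode that runs a collapsing-stage level with goblins, spawned from the game instance's checkpoint list.
; BeginPlay creates the HUD and starts a looping timer, paced by level time over chunk count, that collapses random stage chunks.
; Destroyed chunks advance HUD progress and eventually trigger LevelComplete on the player controller.
; Goblin deaths prune the alive list; an empty list only prints a loss message, with no lose screen called.
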(event `Cleanup HUD`
  ;[0 0 0] HUD Cleanup
  (`Widget.RemoveFromParent` (`self.HUD`)))

(event `self.ReceiveBeginPlay`
  (bind (_stage_ref _stage_ref_2) (`self.Stage Ref`))
  (`GameplayStatics.SpawnSound2D` null 1.0 1.0 0.0 null)
  (`|ExecutionSequence`
    (:`then_0`
      ;[0 0 0] Variable Setup
      (bind _returnvalue (`GameplayStatics.GetActorOfClass` null))
      (set `self.Stage Ref` null _returnvalue)
      (bind _asbp_game_instance (cast `` (`GameplayStatics.GetGameInstance`)))
      (set `self.As BP Game Instance` null _asbp_game_instance))
    (:`then_1`
      ;[0 0 0] HUD Setup
      (`/Engine/EditorBlueprintResources/StandardMacros.IsValid` (`self.HUD`)
        (:`Is Valid`
          ;;[0 0 0] Remove Old HUD
          (`self.Cleanup HUD`))
        (:`Is Not Valid`
          _))
      ;;[0 0 0] Initialize New HUD
      (bind _returnvalue_2 (`|CreateWidget` "/Game/Taylor/UI/HUD/WBP_HUD.WBP_HUD_C"))
      (bind _output_get (set `self.HUD` _returnvalue_2))
      (`UserWidget.AddToViewport` _output_get 0))
    (:`then_2`
      ;[0 0 0] Spawn Goblins from CheckpointGoblins
      (for (_array_element _array_index) (`/Game/Taylor/Mechanics/ToDelete/GM_Gameplay.Checkpoint Goblins` (`.As BP Game Instance` (`self.As BP Game Instance`)))
        (bind _returnvalue_3 (`|SpawnActorFromClass` null (`KismetMathLibrary.MakeTransform` (0.0 0.0 100.0)) "AdjustIfPossibleButAlwaysSpawn" "MultiplyWithRoot" null null))
        (bind (_color _name) (break `` _array_element))
        (set `/Game/Taylor/Mechanics/ToDelete/GM_Gameplay.Color` _color _returnvalue_3)
        (set `/Game/Taylor/Mechanics/ToDelete/GM_Gameplay.Name` _name _returnvalue_3)
        (set `/Game/Taylor/Mechanics/ToDelete/GM_Gameplay.ID` _array_index _returnvalue_3)))
    (:`then_3`
      ;[1 1 0] DEBUG
      (if (> (`/Game/Taylor/Mechanics/ToDelete/GM_Gameplay.ChunksToFall` (`.Stage Ref` (`self.Stage Ref`))) 0)
        ;[0 0 0] Determine Collapse Frequency
        (set `self.Collapse Interval` (`KismetMathLibrary.FClamp` (/ (`/Game/Taylor/Mechanics/ToDelete/GM_Gameplay.Level Time In Seconds` _stage_ref_2) (`/Game/Taylor/Mechanics/ToDelete/GM_Gameplay.ChunksToFall` _stage_ref_2)) 1.0 10.0))
        ;[0 0 0] Set Repeating Collapse Timer
        (bind _returnvalue_4 (`KismetSystemLibrary.K2_SetTimerDelegate` (delegate `Trigger Collapse`) (`self.Collapse Interval`) true))
        (set `self.Timer Handle` _returnvalue_4)
        (else
          (`KismetSystemLibrary.PrintText` "ERROR: ChunksToFall is 0" true true (struct :`A` 1.0)))))))

(event `On Chunk Destroyed`
  (bind _collapse_index (`/Game/Taylor/Mechanics/ToDelete/GM_Gameplay.Collapse Index` (`.Stage Ref` (`self.Stage Ref`))))
  ;[0 0 0 1 24] On Chunk Destroyed
  ;;[0 0 0] Remove Chunk from Arrays
  (`KismetArrayLibrary.Array_Remove` (`/Game/Taylor/Mechanics/ToDelete/GM_Gameplay.Mesh Components` (`.Stage Ref` (`self.Stage Ref`))) _collapse_index)
  (`KismetArrayLibrary.Array_Remove` (`/Game/Taylor/Mechanics/ToDelete/GM_Gameplay.Stage Meshes` (`.Stage Ref` (`self.Stage Ref`))) _collapse_index)
  ;;[0 0 0] Update Number of Fallen Chunks
  (`/Engine/EditorBlueprintResources/StandardMacros.IncrementInt` (`self.Chunks Fallen`)
    (:`  `
      ;;[0 0 0] Update Level Progress (for HUD)
      (set `self.Level Progress` (`KismetMathLibrary.FClamp` (/ (`KismetMathLibrary.Conv_IntToDouble` (`self.Chunks Fallen`)) (`KismetMathLibrary.Conv_IntToDouble` (`/Game/Taylor/Mechanics/ToDelete/GM_Gameplay.ChunksToFall` (`.Stage Ref` (`self.Stage Ref`)))))))
      (`KismetSystemLibrary.Delay` 0.2)
      ;;[0 0 0] Checks If Level Complete
      (if (>= (`self.Chunks Fallen`) (`/Game/Taylor/Mechanics/ToDelete/GM_Gameplay.ChunksToFall` (`.Stage Ref` (`self.Stage Ref`))))
        ;;[0 0 0] End Level
        (`KismetSystemLibrary.K2_ClearAndInvalidateTimerHandle` (`self.Timer Handle`))
        (bind _asbp_player_controller (cast `` (`GameplayStatics.GetPlayerController` 0)))
        (`self.Level Complete` _asbp_player_controller)))))

(event `Trigger Collapse`
  ;[0 0 0 1 24] Stage Collapse Logic
  ;;[0 0 0] Select Next Chunk
  (`self.Get Random Index` (`.Stage Ref` (`self.Stage Ref`)))
  ;;[0 0 0] Tell Stage to Collapse Mesh
  (`self.Collapse Mesh` (`.Stage Ref` (`self.Stage Ref`))))

(event `self.GoblinDied`
  (params (Name :type Name))
  ;[0 0 0 1 24] Goblin Death
  ;;[0 0 0] Remove Goblin From Array
  (for (_array_element _array_index) (`/Game/Taylor/Mechanics/ToDelete/GM_Gameplay.Alive Goblins` (`.As BP Game Instance` (`self.As BP Game Instance`)))
    (if (== Name (`.Name_16_E2775B3A4FF36E521EE9F084E858EA4F` (break `` _array_element)))
      (`KismetArrayLibrary.Array_Remove` (`/Game/Taylor/Mechanics/ToDelete/GM_Gameplay.Alive Goblins` (`.As BP Game Instance` (`self.As BP Game Instance`))) _array_index)))
  ;;[0 0 0] Lose Condition
  (if (`KismetArrayLibrary.Array_IsEmpty` (`/Game/Taylor/Mechanics/ToDelete/GM_Gameplay.Alive Goblins` (`.As BP Game Instance` (`self.As BP Game Instance`))))
    (`KismetSystemLibrary.PrintString` "You Lose!" true true (struct :`R` 1.0 :`G` 1.0 :`B` 1.0 :`A` 1.0) 10.0)
    ;;;[0 0 0] go to PlayerController & call a function to create LoseGame Widget
    (cast `` (`GameplayStatics.GetPlayerController` 0))))

(fn `UserConstructionScript`)