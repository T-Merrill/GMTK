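; Vampire jam game mode that tracks collected blood against a nightly quota.
; AddBlood increases CurrentBlood by the given amount and prints the new total for debugging.
; A separate UpdateBloodTracker event sets LevelProgress by dividing CurrentBlood by NightQuota, then converting the result to a double.
; AddBlood does not call that event, and nothing in these graphs acts on reaching the quota.
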(event `Update Blood Tracker`
  (set `self.Level Progress` (`KismetMathLibrary.Conv_IntToDouble` (/ (`self.Current Blood`) (`self.Night Quota`)))))

(fn `Add Blood`
  (params (Amount :type Integer))
  (bind _output_get (set `self.Current Blood` (+ (`self.Current Blood`) Amount)))
  ;[1 1 0] DEBUG
  (`KismetSystemLibrary.PrintString` (`KismetStringLibrary.Concat_StrStr` "CurrentBlood = " (`KismetStringLibrary.Conv_IntToString` _output_get))))

(fn `UserConstructionScript`)