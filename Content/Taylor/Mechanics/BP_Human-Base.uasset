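; BP_Human-Base is the base human NPC that walks to a building and can be eaten by the player for blood.
; On BeginPlay it picks a random actor tagged Building and moves to that actor's box component, at a walk speed set in the construction script.
; Capsule overlaps toggle an interact prompt; Interact spawns a blood explosion, adds blood plus bonus to the game instance, then destroys the human.
; Blood-stain decal logic is unfinished and unconnected.
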(event `self.ReceiveBeginPlay`
  ;[0 0 0 1 24] Destination & Movement Logic
  ;;[0 0 0] Pick a random building index & set as destination
  (bind _outactors (`GameplayStatics.GetAllActorsWithTag` "Building"))
  (bind _asbp_building__base (cast `/Game/Taylor/Mechanics/BP_Building-Base` (`|GetArrayItem` _outactors (`KismetMathLibrary.RandomIntegerInRange` 0 (`KismetArrayLibrary.Array_LastIndex` _outactors)))))
  (bind _output_get (set `self.Target Building` _asbp_building__base))
  (`|AIMoveTo` self (`SceneComponent.K2_GetComponentLocation` (`self.GetComponentByClass` _output_get "/Script/Engine.BoxComponent")) null 0.0))

(event `/Game/Taylor/Mechanics/BPI_Interactable.Interact`
  (params (Instigator :type "Actor Object Reference"))
  ;[0 0 0 1 24] Interact Logic
  (`NiagaraFunctionLibrary.SpawnSystemAtLocation` "/Game/Van/Assets/Particles/NS_BloodExplosion.NS_BloodExplosion" (`self.K2_GetActorLocation`))
  (bind _asgi_game_instance (cast `/Game/Taylor/Data/GI_GameInstance` (`GameplayStatics.GetGameInstance`)))
  ;;[0 0 0] Increment CurrentBlood When Eaten
  (`/Game/Taylor/Data/GI_GameInstance.Add Blood` _asgi_game_instance (+ (`/Game/Taylor/Data/GI_GameInstance.BonusBlood` _asgi_game_instance) (`self.Blood Value`)))
  (`self.K2_DestroyActor` self))

(event `self.CapsuleComponent.OnComponentBeginOverlap`
  (params (OverlappedComponent :type "PrimitiveComponent Object Reference") (OtherActor :type "Actor Object Reference") (OtherComp :type "PrimitiveComponent Object Reference") (OtherBodyIndex :type Integer) (bFromSweep :type Boolean) (SweepResult :type "HitResult Structure (by ref)"))
  ;[0 0 0 1 24] Interact Overlay on Overlap
  (if (`self.ActorHasTag` OtherActor "Player")
    (`SceneComponent.SetVisibility` (`self.Interact Prompt`) true false)))

(event `self.CapsuleComponent.OnComponentEndOverlap`
  (params (OverlappedComponent :type "PrimitiveComponent Object Reference") (OtherActor :type "Actor Object Reference") (OtherComp :type "PrimitiveComponent Object Reference") (OtherBodyIndex :type Integer))
  ;[0 0 0 1 24] Interact Overlay on Overlap
  (if (`self.ActorHasTag` OtherActor "Player")
    (`SceneComponent.SetVisibility` (`self.Interact Prompt`) false false)))

(fn `UserConstructionScript`
  (set `CharacterMovementComponent.MaxWalkSpeed` (`self.Walk Speed`) (`self.CharacterMovement`)))