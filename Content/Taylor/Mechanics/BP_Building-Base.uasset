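; Base Blueprint for a building that shelters humans, absorbing them at its door until it reaches capacity.
; An actor tagged Human overlapping the door collider increments the occupant count and is destroyed; filling the building turns three cubes yellow and lights three rect lights.
; When full, it calls RejectFromBuilding, which so far only gathers Building-tagged actors.
; The construction script assigns the building mesh a random material from Colors.
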(event `self.Door Collider.OnComponentBeginOverlap`
  (params (OverlappedComponent :type "PrimitiveComponent Object Reference") (OtherActor :type "Actor Object Reference") (OtherComp :type "PrimitiveComponent Object Reference") (OtherBodyIndex :type Integer) (bFromSweep :type Boolean) (SweepResult :type "HitResult Structure (by ref)"))
  (if (`self.ActorHasTag` OtherActor "Human")
    (set `self.Overlapped Human` OtherActor)
    ;[0 0 0] Check if Building is at Max Capacity
    (if (< (`self.Current Occupants`) (`self.Max Capacity`))
      ;[0 0 0] Space Available - Human Enters & Escapes
      (`/Engine/EditorBlueprintResources/StandardMacros.IncrementInt` (`self.Current Occupants`)
        (:`  `
          ;;[0 0 0] Turn Lights On
          (if (>= (`self.Current Occupants`) (`self.Max Capacity`))
            (`PrimitiveComponent.SetMaterial` (`self.Cube`) 0 "/Game/Taylor/Materials/M_Matte-Yellow.M_Matte-Yellow")
            (`PrimitiveComponent.SetMaterial` (`self.Cube1`) 0 "/Game/Taylor/Materials/M_Matte-Yellow.M_Matte-Yellow")
            (`PrimitiveComponent.SetMaterial` (`self.Cube2`) 0 "/Game/Taylor/Materials/M_Matte-Yellow.M_Matte-Yellow")
            (`LightComponent.SetIntensity` (`self.RectLight`) 2.0)
            (`LightComponent.SetIntensity` (`self.RectLight1`) 2.0)
            (`LightComponent.SetIntensity` (`self.RectLight2`) 2.0))
          (`self.K2_DestroyActor` (`self.Overlapped Human`))))
      (else
        ;[0 0 0] Building Is Full
        (`self.Reject From Building`)))))

(fn `Reject From Building`
  (`GameplayStatics.GetAllActorsWithTag` "Building"))

(fn `UserConstructionScript`
  (`PrimitiveComponent.SetMaterial` (`self.BuildingMesh`) 0 (`|GetArrayItem` (`self.Colors`) (`KismetMathLibrary.RandomIntegerInRange` 0 (`KismetArrayLibrary.Array_LastIndex` (`self.Colors`))))))