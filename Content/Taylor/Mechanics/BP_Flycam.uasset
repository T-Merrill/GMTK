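; Fly camera pawn that hands control back to a stored player pawn through a debug key.
; Releasing F10 runs a Visibility line trace from the camera's location to an end point computed from its scale, not its location, minus a Z offset.
; On a hit, it teleports ExistingPlayer to the impact point and, if that succeeds, player controller 0 possesses that pawn.
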(event Input|KeyboardEvents|DebugKeyF10
  (params (Key :type Key%20Structure :default "None") (ActionValue :type Input%20Action%20Value%20Structure))
  (bind _self self)
  (bind _returnvalue (Transformation|GetActorTransform _self))
  (:Released
    (bind (_outhit _returnvalue_2) (Collision|LineTraceByChannel (.location _returnvalue) (- (.scale _returnvalue) "0.000000,0.000000,500.000000") "TraceTypeQuery1" false 0 "None"))
    (if _returnvalue_2
      (bind _returnvalue_3 (Transformation|SetActorTransform (Variables|Default|GetExisting%20Player) (Math|Conversions|ToTransform(Vector) (.ImpactPoint (Collision|BreakHitResult _outhit))) false true))
      (if _returnvalue_3
        (Pawn|Possess (Game|GetPlayerController 0) (Variables|Default|GetExisting%20Player))))))

(fn ConstructionScript)