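; Gameplay game mode that runs a collapsing-stage level: on BeginPlay it starts music, creates the HUD and spawns goblins from the GameInstance's checkpoint list.
; A looping timer, paced by level time over chunk count, tells BP_Stage to collapse random chunks.
; Destroyed chunks update HUD progress and trigger level completion once enough fall.
; Goblin deaths prune the alive list, and an empty list triggers the player controller's lose flow.
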(event `Cleanup HUD`
  ;[0 0 0] HUD Cleanup
  (`Widget.RemoveFromParent` (`self.HUD`)))

(event `self.ReceiveBeginPlay`
  (bind _stage_ref (`self.Stage Ref`))
  (`GameplayStatics.SpawnSound2D` "/Game/KLE/candygoblin_track_final.candygoblin_track_final" 1.0 1.0 0.0 null)
  (`|ExecutionSequence`
    (:`then_0`
      ;[0 0 0] Variable Setup
      (bind _returnvalue (`GameplayStatics.GetActorOfClass` "/Game/Taylor/Mechanics/BP_Stage.BP_Stage_C"))
      (set `self.Stage Ref` _returnvalue)
      (bind _asbp_game_instance (cast `/Game/Taylor/Data/BP_GameInstance` (`GameplayStatics.GetGameInstance`)))
      (set `self.As BP Game Instance` _asbp_game_instance))
    (:`then_1`
      ;[0 0 0] HUD Setup
      (`/Engine/EditorBlueprintResources/StandardMacros.IsValid` (`self.HUD`)
        (:`Is Valid`
          ;;[0 0 0] Remove Old HUD
          (`self.Cleanup HUD`))
        (:`Is Not Valid`
          _))
      ;;[0 0 0] Initialize New HUD
      (bind _returnvalue_2 (`|CreateWidget` "/Game/Taylor/UI/HUD/WBP_HUD.WBP_HUD_C"))
      (bind _output_get (set `self.HUD` _returnvalue_2))
      (`UserWidget.AddToViewport` _output_get 0))
    (:`then_2`
      ;[0 0 0] Spawn Goblins from CheckpointGoblins
      (for (_array_element _array_index) (`/Game/Taylor/Data/BP_GameInstance.Checkpoint Goblins` (`self.As BP Game Instance`))
        (bind _returnvalue_3 (`|SpawnActorFromClass` "/Game/VanStuff/PlayerTesting/Mechanics/BP_Goblin.BP_Goblin_C" (`KismetMathLibrary.MakeTransform` (0.0 0.0 100.0)) "AdjustIfPossibleButAlwaysSpawn" "MultiplyWithRoot" null null))
        (bind (_color _name) (break `/Game/VanStuff/PlayerTesting/Mechanics/S_GoblinData` _array_element))
        (set `/Game/VanStuff/PlayerTesting/Mechanics/BP_Goblin.Color` _color _returnvalue_3)
        (set `/Game/VanStuff/PlayerTesting/Mechanics/BP_Goblin.Name` _name _returnvalue_3)
        (set `/Game/VanStuff/PlayerTesting/Mechanics/BP_Goblin.ID` _array_index _returnvalue_3)))
    (:`then_3`
      ;[1 1 0] DEBUG
      (if (> (`/Game/Taylor/Mechanics/BP_Stage.ChunksToFall` (`self.Stage Ref`)) 0)
        ;[0 0 0] Determine Collapse Frequency
        (set `self.Collapse Interval` (`KismetMathLibrary.FClamp` (/ (`/Game/Taylor/Mechanics/BP_Stage.Level Time In Seconds` _stage_ref) (`/Game/Taylor/Mechanics/BP_Stage.ChunksToFall` _stage_ref)) 1.0 10.0))
        ;[0 0 0] Set Repeating Collapse Timer
        (bind _returnvalue_4 (`KismetSystemLibrary.K2_SetTimerDelegate` (delegate `Trigger Collapse`) (`self.Collapse Interval`) true))
        (set `self.Timer Handle` _returnvalue_4)
        (else
          (`KismetSystemLibrary.PrintText` "ERROR: ChunksToFall is 0" true true (struct :`A` 1.0)))))))

(event `On Chunk Destroyed`
  (bind _collapse_index (`/Game/Taylor/Mechanics/BP_Stage.Collapse Index` (`self.Stage Ref`)))
  ;[0 0 0 1 24] On Chunk Destroyed
  ;;[0 0 0] Remove Chunk from Arrays
  (`KismetArrayLibrary.Array_Remove` (`/Game/Taylor/Mechanics/BP_Stage.Mesh Components` (`self.Stage Ref`)) _collapse_index)
  (`KismetArrayLibrary.Array_Remove` (`/Game/Taylor/Mechanics/BP_Stage.Stage Meshes` (`self.Stage Ref`)) _collapse_index)
  ;;[0 0 0] Update Number of Fallen Chunks
  (`/Engine/EditorBlueprintResources/StandardMacros.IncrementInt` (`self.Chunks Fallen`)
    (:`  `
      ;;[0 0 0] Update Level Progress (for HUD)
      (set `self.Level Progress` (`KismetMathLibrary.FClamp` (/ (`KismetMathLibrary.Conv_IntToDouble` (`self.Chunks Fallen`)) (`KismetMathLibrary.Conv_IntToDouble` (`/Game/Taylor/Mechanics/BP_Stage.ChunksToFall` (`self.Stage Ref`))))))
      (`KismetSystemLibrary.Delay` 0.2)
      ;;[0 0 0] Checks If Level Complete
      (if (>= (`self.Chunks Fallen`) (`/Game/Taylor/Mechanics/BP_Stage.ChunksToFall` (`self.Stage Ref`)))
        ;;[0 0 0] End Level
        (`KismetSystemLibrary.K2_ClearAndInvalidateTimerHandle` (`self.Timer Handle`))
        (bind _asbp_player_controller (cast `/Game/VanStuff/PlayerTesting/Mechanics/BP_PlayerController` (`GameplayStatics.GetPlayerController` 0)))
        (`/Game/VanStuff/PlayerTesting/Mechanics/BP_PlayerController.Level Complete` _asbp_player_controller)))))

(event `Trigger Collapse`
  ;[0 0 0 1 24] Stage Collapse Logic
  ;;[0 0 0] Select Next Chunk
  (`/Game/Taylor/Mechanics/BP_Stage.Get Random Index` (`self.Stage Ref`))
  ;;[0 0 0] Tell Stage to Collapse Mesh
  (`/Game/Taylor/Mechanics/BP_Stage.Collapse Mesh` (`self.Stage Ref`)))

(event `/Game/VanStuff/PlayerTesting/Mechanics/BPI_GoblinDeath.GoblinDied`
  (params (Name :type Name))
  ;[0 0 0 1 24] Goblin Death
  ;;[0 0 0] Remove Goblin From Array
  (for (_array_element _array_index) (`/Game/Taylor/Data/BP_GameInstance.Alive Goblins` (`self.As BP Game Instance`))
    (if (== Name (`.Name_16_E2775B3A4FF36E521EE9F084E858EA4F` (break `/Game/VanStuff/PlayerTesting/Mechanics/S_GoblinData` _array_element)))
      (`KismetArrayLibrary.Array_Remove` (`/Game/Taylor/Data/BP_GameInstance.Alive Goblins` (`self.As BP Game Instance`)) _array_index)))
  ;;[0 0 0] Lose Condition
  (if (`KismetArrayLibrary.Array_IsEmpty` (`/Game/Taylor/Data/BP_GameInstance.Alive Goblins` (`self.As BP Game Instance`)))
    (`KismetSystemLibrary.PrintString` "You Lose!" true true (struct :`R` 1.0 :`G` 1.0 :`B` 1.0 :`A` 1.0) 10.0)
    ;;;[0 0 0] go to PlayerController & call a function to create LoseGame Widget
    (bind _asbp_player_controller (cast `/Game/VanStuff/PlayerTesting/Mechanics/BP_PlayerController` (`GameplayStatics.GetPlayerController` 0)))
    (`/Game/VanStuff/PlayerTesting/Mechanics/BP_PlayerController.On Lose Game` _asbp_player_controller)))

(fn `UserConstructionScript`)